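; A world-space menu actor that shows a swappable widget and can be picked up and dropped.
; Pickup attaches its root to a given component and Drop detaches it, both keeping the world transform.
; ChangeMenu sets the widget on the Menu component.
; GetMenuLocation returns that component's world transform at unit scale, with roll and pitch offset by a half turn.
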(event EventBeginPlay)

(event Collision|EventActorBeginOverlap
  (params (OtherActor :type Actor%20Object%20Reference)))

(event EventTick
  (params (DeltaSeconds :type Float%20%28single-precision%29)))

(event EventPickup
  (params (AttachTo :type Scene%20Component%20Object%20Reference) (RightHand? :type Boolean))
  (Transformation|AttachComponentToComponent (VehicleSound|GetRootComponent) AttachTo "None" "KeepWorld" "KeepWorld" "KeepWorld" false))

(event EventDrop
  (Transformation|DetachFromActor "KeepWorld" "KeepWorld" "KeepWorld"))

(fn ConstructionScript)

(fn ChangeMenu
  (params (NewWidget :type Host%20Menu%20Object%20Reference))
  (UserInterface|SetWidget (Variables|Default|GetMenu) NewWidget))

(fn GetMenuLocation
  (bind _menu (Variables|Default|GetMenu))
  (bind _returnvalue (Transformation|GetWorldRotation _menu))
  (bind (_roll _pitch _yaw) (Math|Rotator|BreakRotator _returnvalue))
  (return (Math|Transform|MakeTransform (Transformation|GetWorldLocation _menu) (Math|Rotator|MakeRotator (+ _roll 1.8e+02) (+ _pitch 1.8e+02) _yaw) "1.000000,1.000000,1.000000")))